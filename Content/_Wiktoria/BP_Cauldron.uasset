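; BP_Cauldron is an alchemy cauldron actor that shows its brew's state through an on-screen stats widget and the liquid's color.
; On BeginPlay it creates the widget and a dynamic liquid material, then passes its ingredient trigger zone to the CoreAlchemy component.
; CoreAlchemy's OnStateChanged event refreshes the widget and maps temperature, acidity and density to the liquid's red, green and blue channels.
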(event `self.ReceiveBeginPlay`
  (bind _returnvalue (`|CreateWidget` "/Game/_Wiktoria/WBP_CauldronStats.WBP_CauldronStats_C"))
  (bind _output_get (set `self.UI_Reference` _returnvalue))
  (`UserWidget.AddToViewport` _output_get 0)
  (bind _returnvalue_2 (`PrimitiveComponent.CreateDynamicMaterialInstance` (`self.Liquid`) 0 "/Game/_Wiktoria/MI_LiquidCauldron.MI_LiquidCauldron" "None"))
  (set `self.LiquidMaterial` _returnvalue_2)
  (`CoreAlchemyComponent.SetupCauldronTrigger` (`self.CoreAlchemy`) (`self.IngredientTriggerZone`)))

(event `self.CoreAlchemy.OnStateChanged`
  (bind _corealchemy (`self.CoreAlchemy`))
  (bind _corealchemy_2 (`self.CoreAlchemy`))
  (`/Game/_Wiktoria/WBP_CauldronStats.UpdateStatsUI` (`self.UI_Reference`) (`CoreAlchemyComponent.Temperature` _corealchemy) (`CoreAlchemyComponent.Acidity` _corealchemy) (`CoreAlchemyComponent.Density` _corealchemy))
  (`MaterialInstanceDynamic.SetVectorParameterValue` (`self.LiquidMaterial`) "Color" (make `LinearColor` (`KismetMathLibrary.MapRangeClamped` (`KismetMathLibrary.Conv_IntToDouble` (`CoreAlchemyComponent.Temperature` _corealchemy_2)) -4.0 4.0 0.0 1.0) (`KismetMathLibrary.MapRangeClamped` (`KismetMathLibrary.Conv_IntToDouble` (`CoreAlchemyComponent.Acidity` _corealchemy_2)) -4.0 4.0 0.0 1.0) (`KismetMathLibrary.MapRangeClamped` (`KismetMathLibrary.Conv_IntToDouble` (`CoreAlchemyComponent.Density` _corealchemy_2)) -4.0 4.0 0.0 1.0) 1.0)))

(fn `UserConstructionScript`)