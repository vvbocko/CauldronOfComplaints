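; BP_TestInteractionActor is a test interactable that toggles a point light when interacted with.
; It handles interface events for focus and interaction: focus sets custom depth rendering on the cube and prints the focus state.
; Interact flips a boolean to show or hide the light, and a getter exposes the actor's widget reference.
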(event `/Game/Blueprints/BPI_Interaction.Interface_ToggleFocus`
  (params (Focus :type Boolean))
  (`PrimitiveComponent.SetRenderCustomDepth` (`self.Cube`) Focus)
  (`KismetSystemLibrary.PrintString` (`KismetStringLibrary.Conv_BoolToString` Focus) true true (struct :`R` 0.102642 :`B` 1.0 :`A` 1.0)))

(event `/Game/Blueprints/BPI_Interaction.InterfaceInteract`
  (`self.Interact`))

(event `Interact`
  (bind _pointlight (`self.PointLight`))
  (bind _output_get (set `self.InteractToggle` (not (`self.InteractToggle`))))
  (if _output_get
    (`SceneComponent.SetVisibility` _pointlight true false)
    (else
      (`SceneComponent.SetVisibility` _pointlight false false))))

(fn `GetInteractionWidgetRef`
  (returns (WidgetReference :type "WidgetComponent Object Reference"))
  (return (`self.Widget`)))

(fn `UserConstructionScript`)