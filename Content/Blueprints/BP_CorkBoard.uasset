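; BP_CorkBoard is a board actor that fills itself with three random paper orders when play begins.
; It shuffles the row names of DT_OrdersList and takes the first three, so each pick comes from a different row.
; For each row found, it spawns a BP_PaperComplaint at the matching slot component's location and rotation, passing the row in as its order data.
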(event `self.ReceiveBeginPlay`
  (bind _outrownames (`DataTableFunctionLibrary.GetDataTableRowNames` "/Game/Blueprints/DT_OrdersList.DT_OrdersList"))
  (`KismetArrayLibrary.Array_Shuffle` _outrownames)
  (for _index (range 3)
    (bind _returnvalue (`|GetDataTableRow` "/Game/Blueprints/DT_OrdersList.DT_OrdersList" (`|GetArrayItem` _outrownames _index))
      (:`then`
        (bind (_returnvalue_location _returnvalue_rotation) (`KismetMathLibrary.BreakTransform` (`SceneComponent.K2_GetComponentToWorld` (`|GetArrayItem` (`|MakeArray` (`self.Slot_1`) (`self.Slot_2`) (`self.Slot_3`)) _index))))
        (`|SpawnActorFromClass` "/Game/Blueprints/BP_PaperComplaint.BP_PaperComplaint_C" (`KismetMathLibrary.MakeTransform` _returnvalue_location _returnvalue_rotation) "AlwaysSpawn" "MultiplyWithRoot" null _returnvalue null)))))

(fn `UserConstructionScript`)