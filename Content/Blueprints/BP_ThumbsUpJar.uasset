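; BP_ThumbsUpJar is an interactable jar actor that shows a thumbs-up tally based on a success count.
; UpdateGoodJar reveals one of three static meshes for counts one to three, with debug prints.
; Interface focus toggles custom depth on the jar and updates its WBP_InteractionJars widget with a Polish label and the count plus a fixed offset.
; GetInteractionWidgetRef exposes that widget component.
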(event `UpdateGoodJar`
  (params (SuccessCount :type Integer))
  (bind _staticmesh1 (`self.StaticMesh1`))
  (bind _staticmesh2 (`self.StaticMesh2`))
  (bind _staticmesh3 (`self.StaticMesh3`))
  (`KismetSystemLibrary.PrintString` (`KismetStringLibrary.Conv_IntToString` SuccessCount) true true (struct :`R` 1.0 :`B` 0.003656 :`A` 1.0))
  (switch `int` SuccessCount
    (:`1`
      (`SceneComponent.SetVisibility` _staticmesh1 true false)
      (`KismetSystemLibrary.PrintString` (`KismetSystemLibrary.GetDisplayName` _staticmesh1) true true (struct :`R` 1.0 :`B` 0.003656 :`A` 1.0)))
    (:`2`
      (`SceneComponent.SetVisibility` _staticmesh2 true false)
      (`KismetSystemLibrary.PrintString` (`KismetSystemLibrary.GetDisplayName` _staticmesh2) true true (struct :`R` 1.0 :`B` 0.003656 :`A` 1.0)))
    (:`3`
      (`SceneComponent.SetVisibility` _staticmesh3 true false)
      (`KismetSystemLibrary.PrintString` (`KismetSystemLibrary.GetDisplayName` _staticmesh3) true true (struct :`R` 1.0 :`B` 0.003656 :`A` 1.0)))))

(event `/Game/Blueprints/BPI_Interaction.Interface_ToggleFocus`
  (params (Focus :type Boolean))
  (`PrimitiveComponent.SetRenderCustomDepth` (`self.Jar`) Focus)
  (bind _aswbp_interaction_jars (cast `/Game/UI/WBP_InteractionJars` (`WidgetComponent.GetUserWidgetObject` (`self.Widget`))))
  (`/Game/UI/WBP_InteractionJars.UpdateWidgetInfo` _aswbp_interaction_jars (`|FormatText` "{Thumbs}:   {Total}" "Kciuki w górę" (`KismetTextLibrary.Conv_IntToText` (+ 13 (stale `UpdateGoodJar` SuccessCount))))))

(fn `GetInteractionWidgetRef`
  (returns (WidgetReference :type "WidgetComponent Object Reference"))
  (return (`self.Widget`)))

(fn `UserConstructionScript`)