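; Actor component that lets the player focus and trigger BP_InteractionArea actors by looking at them.
; Every tick, a Visibility line trace from the player camera, limited by ReachLength, updates the focused actor and toggles the area's focus.
; TryInteracting sends an interface interact message to the focused area's parent actor when its InteractDuration is not positive.
; Timed interactions have no handling here.
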(event `self.ReceiveTick`
  (params (DeltaSeconds :type "Float (single-precision)"))
  (`self.Trace`))

(event `TryInteracting`
  (params (In :type Boolean))
  (if In
    (if (`self.IsTracingInteractionArea`)
      (bind _output_get (set `self.Interact Duration` (`/Game/Blueprints/BP_InteractionArea.InteractDuration` (`self.FocusedInteractionArea`))))
      (if (not (> _output_get 0.0))
        (`self.Interact` (`self.FocusedInteractionArea`))))))

(event `Interact`
  (params (InteractionArea :type "/Game/Blueprints/BP_InteractionArea Object Reference"))
  (message `/Game/Blueprints/BPI_Interaction.InterfaceInteract` (`Actor.GetParentActor` InteractionArea)))

(fn `Trace`
  (bind _returnvalue (`GameplayStatics.GetPlayerCameraManager` 0))
  (bind _returnvalue_2 (`Actor.K2_GetActorLocation` _returnvalue))
  (bind (_outhit _returnvalue_3) (`KismetSystemLibrary.LineTraceSingle` _returnvalue_2 (+ _returnvalue_2 (* (`KismetMathLibrary.GetForwardVector` (`Actor.K2_GetActorRotation` _returnvalue)) (`self.ReachLength`))) "TraceTypeQuery1"))
  (if _returnvalue_3
    (bind (_bblockinghit _binitialoverlap _time _distance _location _impactpoint _normal _impactnormal _physmat _hitactor) (`GameplayStatics.BreakHitResult` _outhit))
    (if (!= (`self.FocusedActor`) _hitactor)
      (set `self.FocusedActor` _hitactor)
      (`self.TraceInteractionArea` (== (`GameplayStatics.GetObjectClass` _hitactor) "/Game/Blueprints/BP_InteractionArea.BP_InteractionArea_C")))
    (else
      (`self.TraceInteractionArea` false))))

(fn `TraceInteractionArea`
  (params (isTraceOn :type Boolean))
  (if isTraceOn
    (if (`self.IsTracingInteractionArea`)
      (`/Game/Blueprints/BP_InteractionArea.ToggleFocus` (`self.FocusedInteractionArea`) false))
    (bind _asbp_interaction_area (cast `/Game/Blueprints/BP_InteractionArea` (`self.FocusedActor`)))
    (bind _output_get (set `self.FocusedInteractionArea` _asbp_interaction_area))
    (`/Game/Blueprints/BP_InteractionArea.ToggleFocus` _output_get true)
    (set `self.IsTracingInteractionArea` true)
    (elif (`self.IsTracingInteractionArea`)
      (set `self.IsTracingInteractionArea` false)
      (`/Game/Blueprints/BP_InteractionArea.ToggleFocus` (`self.FocusedInteractionArea`) false)
      (set `self.FocusedActor` null)
      (set `self.FocusedInteractionArea` null))))