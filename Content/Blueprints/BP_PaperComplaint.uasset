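; BP_PaperComplaint is an interactable paper complaint, linked to a cork board, that the player can read.
; Interface events toggle a custom-depth highlight on the paper when focused and, on interact, open the complaint view and hide the cork board's arrow.
; The view is a WBP_OrderView widget built from the paper's order data, shown with UI-only input, a visible cursor and the game paused.
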(event `/Game/Blueprints/BPI_Interaction.Interface_ToggleFocus`
  (params (Focus :type Boolean))
  (`PrimitiveComponent.SetRenderCustomDepth` (`self.Paper`) Focus))

(event `/Game/Blueprints/BPI_Interaction.InterfaceInteract`
  (params (Player :type "/Game/FirstPerson/Blueprints/BP_FirstPersonCharacter Object Reference"))
  (`self.ShowComplaintUI`)
  (`/Game/Blueprints/BP_CorkBoard.HideArrow` (`self.CorkBoardRef`)))

(event `ShowComplaintUI`
  (bind _returnvalue (`GameplayStatics.GetPlayerController` 0))
  (bind _returnvalue_2 (`|CreateWidget` "/Game/UI/WBP_OrderView.WBP_OrderView_C" null (`self.PaperOrderData`) self))
  (`UserWidget.AddToViewport` _returnvalue_2 0)
  (`WidgetBlueprintLibrary.SetInputMode_UIOnlyEx` _returnvalue _returnvalue_2)
  (set `PlayerController.bShowMouseCursor` true _returnvalue)
  (`GameplayStatics.SetGamePaused` true))

(fn `GetInteractionWidgetRef`
  (returns (WidgetReference :type "WidgetComponent Object Reference"))
  (return (`self.Widget`)))

(fn `UserConstructionScript`)