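; Interactable jar actor representing the "bad" thumbs-down jar, holding three thumb meshes.
; UpdateBadJar takes a success count from 0 to 2 and hides the matching thumb, starting with Thumb3.
; Focus toggling through an interface switches custom depth on the jar and sets its interaction widget to bad-jar info.
; A getter exposes that widget component to other Blueprints.
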(event `UpdateBadJar`
  (params (SuccessCount :type Integer))
  (switch `int` SuccessCount
    (:`0`
      (`SceneComponent.SetVisibility` (`self.Thumb_3`) false false))
    (:`1`
      (`SceneComponent.SetVisibility` (`self.Thumb_2`) false false))
    (:`2`
      (`SceneComponent.SetVisibility` (`self.Thumb_1`) false false))))

(event `/Game/Blueprints/BPI_Interaction.Interface_ToggleFocus`
  (params (Focus :type Boolean))
  (`PrimitiveComponent.SetRenderCustomDepth` (`self.Jar`) Focus)
  (bind _aswbp_interaction_jars (cast `/Game/UI/WBP_InteractionJars` (`WidgetComponent.GetUserWidgetObject` (`self.Widget`))))
  (`/Game/UI/WBP_InteractionJars.UpdateWidgetInfo` _aswbp_interaction_jars false false))

(fn `GetInteractionWidgetRef`
  (returns (WidgetReference :type "WidgetComponent Object Reference"))
  (return (`self.Widget`)))

(fn `UserConstructionScript`)