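; Game mode for an alchemy game that tracks order results and ends the session once the maximum order count is reached.
; RegisterOrderResult counts every order, and on success increments the successful count and passes it to both the thumbs-down and thumbs-up jar actors.
; Failed orders update neither jar.
; EndGame shows the game-over widget, switches to UI-only input with a visible cursor, and pauses the game.
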(event `RegisterOrderResult`
  (params (WasOrderSuccesful :type Boolean))
  (if WasOrderSuccesful
    (bind _result (`/Engine/EditorBlueprintResources/StandardMacros.IncrementInt` (`self.SuccesfulOrdersCount`))
      (:`  `
        (bind _output_get (set `self.SuccesfulOrdersCount` _result))
        ; Change
        (bind _returnvalue (`GameplayStatics.GetActorOfClass` "/Game/Blueprints/BP_ThumbsDownJar.BP_ThumbsDownJar_C"))
        (`/Game/Blueprints/BP_ThumbsDownJar.UpdateBadJar` _returnvalue _output_get)
        ; Change
        (bind _returnvalue_2 (`GameplayStatics.GetActorOfClass` "/Game/Blueprints/BP_ThumbsUpJar.BP_ThumbsUpJar_C"))
        (`/Game/Blueprints/BP_ThumbsUpJar.UpdateGoodJar` _returnvalue_2 _output_get))))
  (bind _result_2 (`/Engine/EditorBlueprintResources/StandardMacros.IncrementInt` (`self.TotalOrdersCount`))
    (:`  `
      (bind _output_get_2 (set `self.TotalOrdersCount` _result_2))
      (if (== _output_get_2 (`self.MaxOrderCount`))
        (`self.EndGame`)))))

(event `EndGame`
  (bind _returnvalue (`GameplayStatics.GetPlayerController` 0))
  (bind _returnvalue_2 (`|CreateWidget` "/Game/UI/WBP_GameOverMenu.WBP_GameOverMenu_C"))
  (`UserWidget.AddToViewport` _returnvalue_2 0)
  (`WidgetBlueprintLibrary.SetInputMode_UIOnlyEx` _returnvalue _returnvalue_2)
  (set `PlayerController.bShowMouseCursor` true _returnvalue)
  (`GameplayStatics.SetGamePaused` true))

(fn `UserConstructionScript`
  (`parent.UserConstructionScript`))