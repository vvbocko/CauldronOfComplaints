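; BP_Ingr_PhoenixFeather is a phoenix feather ingredient pickup for the cauldron feature, with physics off at BeginPlay.
; Interface focus events toggle custom depth rendering on its mesh.
; On interact, if the player holds nothing, it disables collision, snaps the mesh component to the player's HoldPosition, shows the drop UI and registers itself as HeldItem.
; It also exposes its interaction widget through a getter.
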(event `self.ReceiveBeginPlay`
  (`PrimitiveComponent.SetSimulatePhysics` (`self.MeshComponent`) false))

(event `self.Interface_ToggleFocus`
  (params (Focus :type Boolean))
  (`PrimitiveComponent.SetRenderCustomDepth` (`self.MeshComponent`) Focus))

(event `self.InterfaceInteract`
  (params (Player :type "/Game/FirstPerson/Blueprints/BP_FirstPersonCharacter Object Reference"))
  (bind _meshcomponent (`self.MeshComponent`))
  (`/Engine/EditorBlueprintResources/StandardMacros.IsValid` (`/Game/FirstPerson/Blueprints/BP_FirstPersonCharacter.HeldItem` Player)
    (:`Is Not Valid`
      (`PrimitiveComponent.SetSimulatePhysics` _meshcomponent false)
      (`PrimitiveComponent.SetCollisionEnabled` _meshcomponent "NoCollision")
      (`SceneComponent.K2_SetRelativeLocationAndRotation` :`self` _meshcomponent)
      (`/Game/UI/WBP_PlayerHUD.ShowDropUI` (`/Game/FirstPerson/Blueprints/BP_FirstPersonCharacter.HUDReference` Player))
      (`SceneComponent.K2_AttachToComponent` _meshcomponent (`/Game/FirstPerson/Blueprints/BP_FirstPersonCharacter.HoldPosition` Player) "None" "SnapToTarget" "SnapToTarget" "KeepWorld" true)
      (set `/Game/FirstPerson/Blueprints/BP_FirstPersonCharacter.HeldItem` self Player))))

(fn `GetInteractionWidgetRef`
  (returns (WidgetReference :type "WidgetComponent Object Reference"))
  (return (`self.Widget`)))

(fn `UserConstructionScript`)