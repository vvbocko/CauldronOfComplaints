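; Interactable alchemy cauldron that takes the player's held ingredient and displays its brew state.
; Interacting releases the held ingredient above the pot with physics on, toward the trigger zone registered with the CoreAlchemy component.
; CoreAlchemy state changes refresh a stats widget and map temperature, acidity and density to the liquid material's RGB color.
; Focus toggles custom depth on the cauldron mesh; the clean/dirty material toggle is unconnected.
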(event `self.ReceiveBeginPlay`
  (bind _returnvalue (`|CreateWidget` "/Game/UI/WBP_CauldronStats.WBP_CauldronStats_C"))
  (bind _output_get (set `self.UI_Reference` _returnvalue))
  (`UserWidget.AddToViewport` _output_get 0)
  (bind _returnvalue_2 (`PrimitiveComponent.CreateDynamicMaterialInstance` (`self.Liquid`) 0 "/Game/Blueprints/Cauldron/MI_LiquidCauldron.MI_LiquidCauldron" "None"))
  (set `self.LiquidMaterial` _returnvalue_2)
  (`CoreAlchemyComponent.SetupCauldronTrigger` (`self.CoreAlchemy`) (`self.IngredientTriggerZone`)))

(event `self.CoreAlchemy.OnStateChanged`
  (bind _corealchemy (`self.CoreAlchemy`))
  (bind _corealchemy_2 (`self.CoreAlchemy`))
  (`/Game/UI/WBP_CauldronStats.UpdateStatsUI` (`self.UI_Reference`) (`CoreAlchemyComponent.Temperature` _corealchemy) (`CoreAlchemyComponent.Acidity` _corealchemy) (`CoreAlchemyComponent.Density` _corealchemy))
  (`MaterialInstanceDynamic.SetVectorParameterValue` (`self.LiquidMaterial`) "Color" (make `LinearColor` (`KismetMathLibrary.MapRangeClamped` (`KismetMathLibrary.Conv_IntToDouble` (`CoreAlchemyComponent.Temperature` _corealchemy_2)) -4.0 4.0 0.0 1.0) (`KismetMathLibrary.MapRangeClamped` (`KismetMathLibrary.Conv_IntToDouble` (`CoreAlchemyComponent.Acidity` _corealchemy_2)) -4.0 4.0 0.0 1.0) (`KismetMathLibrary.MapRangeClamped` (`KismetMathLibrary.Conv_IntToDouble` (`CoreAlchemyComponent.Density` _corealchemy_2)) -4.0 4.0 0.0 1.0) 1.0)))

(event `/Game/Blueprints/BPI_Interaction.Interface_ToggleFocus`
  (params (Focus :type Boolean))
  (`PrimitiveComponent.SetRenderCustomDepth` (`self.Cauldron`) Focus))

(event `/Game/Blueprints/BPI_Interaction.InterfaceInteract`
  (params (Player :type "/Game/FirstPerson/Blueprints/BP_FirstPersonCharacter Object Reference"))
  (bind _helditem (`/Game/FirstPerson/Blueprints/BP_FirstPersonCharacter.HeldItem` Player))
  (`/Engine/EditorBlueprintResources/StandardMacros.IsValid` _helditem
    (:`Is Valid`
      (bind _asalchemy_ingredient (cast `AlchemyIngredient` _helditem))
      (`self.K2_DetachFromActor` _asalchemy_ingredient "KeepWorld" "KeepWorld" "KeepWorld")
      (`self.K2_SetActorLocation` _asalchemy_ingredient (+ (`SceneComponent.K2_GetComponentLocation` (`self.Cauldron`)) (0.0 0.0 80.0)) false false)
      (bind _meshcomponent (`AlchemyIngredient.MeshComponent` _asalchemy_ingredient))
      (`PrimitiveComponent.SetSimulatePhysics` _meshcomponent true)
      (`PrimitiveComponent.SetCollisionProfileName` _meshcomponent "PhysicsActor" true)
      (set `/Game/FirstPerson/Blueprints/BP_FirstPersonCharacter.HeldItem` null Player))))

(event `Interact`)

(fn `GetInteractionWidgetRef`
  (returns (WidgetReference :type "WidgetComponent Object Reference"))
  (return (`self.Widget`)))

(fn `UserConstructionScript`)