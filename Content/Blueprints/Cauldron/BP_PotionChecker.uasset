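; BP_PotionChecker is an interactable that judges the player's held full vial against their active customer order.
; Interacting hides an arrow mesh and, if an order paper exists, compares temperature, acid and density after a brief delay.
; Either result shows a pausing feedback pop-up, then destroys vial and paper and clears the order and HUD.
; Focus toggles custom depth on its Widget; no wallet update happens here despite a comment.
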(event `/Game/Blueprints/BPI_Interaction.Interface_ToggleFocus`
  (params (Focus :type Boolean))
  (`PrimitiveComponent.SetRenderCustomDepth` (`self.Widget`) Focus))

(event `/Game/Blueprints/BPI_Interaction.InterfaceInteract`
  (params (Player :type "/Game/FirstPerson/Blueprints/BP_FirstPersonCharacter Object Reference"))
  (`self.CheckPotion` Player)
  (`SceneComponent.SetVisibility` (`self.SM_FieldArrow`) false false))

(event `CheckPotion`
  (params (FirstPersonCharacter :type "/Game/FirstPerson/Blueprints/BP_FirstPersonCharacter Object Reference"))
  (bind (_title _description _temprequired _acidrequired _densrequired) (break `/Game/Blueprints/S_ClientsOrder` (`/Game/FirstPerson/Blueprints/BP_FirstPersonCharacter.ActiveOrder` FirstPersonCharacter)))
  (bind _asbp_vial_full (cast `/Game/Blueprints/Cauldron/BP_Vial_Full` (`/Game/FirstPerson/Blueprints/BP_FirstPersonCharacter.HeldItem` FirstPersonCharacter)))
  (`/Engine/EditorBlueprintResources/StandardMacros.IsValid` (`/Game/FirstPerson/Blueprints/BP_FirstPersonCharacter.ActiveOrderPaperRef` FirstPersonCharacter)
    (:`Is Valid`
      (`KismetSystemLibrary.Delay` 0.2)
      (if (and (== (`/Game/Blueprints/Cauldron/BP_Vial_Full.ContainedTemp` _asbp_vial_full) _temprequired) (and (== (`/Game/Blueprints/Cauldron/BP_Vial_Full.ContainedAcid` _asbp_vial_full) _acidrequired) (== (`/Game/Blueprints/Cauldron/BP_Vial_Full.ContainedDens` _asbp_vial_full) _densrequired)))
        (`self.CorrectPotion`)
        (else
          (`self.IncorrectPotion`))))))

(event `CorrectPotion`
  ; Increment Wallet (wallet will update thumbsjar)
  (`self.ShowFeedback` "Sukces! Klient cofnie swoją skargę i kciuka w dół.")
  ; Finish Order
  (`self.K2_DestroyActor` (stale `CheckPotion` _asbp_vial_full) :!label _label)
  (set `/Game/FirstPerson/Blueprints/BP_FirstPersonCharacter.HeldItem` null (stale `CheckPotion` FirstPersonCharacter))
  (set `/Game/FirstPerson/Blueprints/BP_FirstPersonCharacter.ActiveOrder` (struct) (stale `CheckPotion` FirstPersonCharacter))
  (`/Game/UI/WBP_PlayerHUD.HideActiveOrderUI` (`/Game/FirstPerson/Blueprints/BP_FirstPersonCharacter.HUDReference` (stale `CheckPotion` FirstPersonCharacter)))
  (bind _activeorderpaperref (`/Game/FirstPerson/Blueprints/BP_FirstPersonCharacter.ActiveOrderPaperRef` (stale `CheckPotion` FirstPersonCharacter)))
  (`/Engine/EditorBlueprintResources/StandardMacros.IsValid` _activeorderpaperref
    (:`Is Valid`
      (`self.K2_DestroyActor` _activeorderpaperref)
      (set `/Game/FirstPerson/Blueprints/BP_FirstPersonCharacter.ActiveOrderPaperRef` null (stale `CheckPotion` FirstPersonCharacter)))))

(event `ShowFeedback`
  (params (FeedbackDescription :type Text))
  (bind _returnvalue (`GameplayStatics.GetPlayerController` 0))
  (bind (_title _description _temprequired _acidrequired _densrequired) (break `/Game/Blueprints/S_ClientsOrder` (`/Game/FirstPerson/Blueprints/BP_FirstPersonCharacter.ActiveOrder` (stale `CheckPotion` FirstPersonCharacter))))
  (bind _returnvalue_2 (`|CreateWidget` "/Game/UI/WBP_FeedbackPopUp.WBP_FeedbackPopUp_C" null FeedbackDescription (and (== (`/Game/Blueprints/Cauldron/BP_Vial_Full.ContainedTemp` (stale `CheckPotion` _asbp_vial_full)) _temprequired) (and (== (`/Game/Blueprints/Cauldron/BP_Vial_Full.ContainedAcid` (stale `CheckPotion` _asbp_vial_full)) _acidrequired) (== (`/Game/Blueprints/Cauldron/BP_Vial_Full.ContainedDens` (stale `CheckPotion` _asbp_vial_full)) _densrequired)))))
  (`UserWidget.AddToViewport` _returnvalue_2 0)
  (`WidgetBlueprintLibrary.SetInputMode_UIOnlyEx` _returnvalue _returnvalue_2)
  (set `PlayerController.bShowMouseCursor` true _returnvalue)
  (`GameplayStatics.SetGamePaused` true))

(event `IncorrectPotion`
  ; Show feedback to player
  (`self.ShowFeedback` "Ups! Eliksir nie spełnił wymagań klienta...")
  (goto _label))

(fn `GetInteractionWidgetRef`
  (returns (WidgetReference :type "WidgetComponent Object Reference"))
  (return (`self.Widget`)))

(fn `UserConstructionScript`)