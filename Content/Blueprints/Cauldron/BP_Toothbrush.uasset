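; BP_Toothbrush is an interactable toothbrush item that the player can pick up and hold.
; Focus toggles custom depth rendering on the toothbrush component, and a getter exposes its interaction widget.
; Interacting with an empty hand disables physics and collision, snaps the component to the player's HoldPosition, and registers the actor as HeldItem.
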(event `/Game/Blueprints/BPI_Interaction.Interface_ToggleFocus`
  (params (Focus :type Boolean))
  (`PrimitiveComponent.SetRenderCustomDepth` (`self.Toothbrush`) Focus))

(event `/Game/Blueprints/BPI_Interaction.InterfaceInteract`
  (params (Player :type "/Game/FirstPerson/Blueprints/BP_FirstPersonCharacter Object Reference"))
  (bind _toothbrush (`self.Toothbrush`))
  (`/Engine/EditorBlueprintResources/StandardMacros.IsValid` (`/Game/FirstPerson/Blueprints/BP_FirstPersonCharacter.HeldItem` Player)
    (:`Is Not Valid`
      (`PrimitiveComponent.SetSimulatePhysics` _toothbrush false)
      (`PrimitiveComponent.SetCollisionEnabled` _toothbrush "NoCollision")
      (`SceneComponent.K2_AttachToComponent` _toothbrush (`/Game/FirstPerson/Blueprints/BP_FirstPersonCharacter.HoldPosition` Player) "None" "SnapToTarget" "SnapToTarget" "KeepWorld" true)
      (set `/Game/FirstPerson/Blueprints/BP_FirstPersonCharacter.HeldItem` self Player))))

(fn `GetInteractionWidgetRef`
  (returns (WidgetReference :type "WidgetComponent Object Reference"))
  (return (`self.Widget`)))

(fn `UserConstructionScript`)