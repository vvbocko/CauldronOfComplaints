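; BP_Vial_Full is an interactable vial of cauldron liquid that the player can pick up and hold.
; On BeginPlay it creates a dynamic instance of MI_LiquidCauldron on the Vial mesh and tints it with the saved liquid color.
; Focus toggles custom depth on the mesh.
; Interacting with empty hands disables physics and collision, attaches the mesh to the player's hold position, shows the drop UI and sets the held item.
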(event `self.ReceiveBeginPlay`
  (bind _returnvalue (`PrimitiveComponent.CreateDynamicMaterialInstance` (`self.Vial`) 0 "/Game/Blueprints/Cauldron/MI_LiquidCauldron.MI_LiquidCauldron" "None"))
  (`MaterialInstanceDynamic.SetVectorParameterValue` _returnvalue "Color" (`self.SavedLiquidColor`)))

(event `/Game/Blueprints/BPI_Interaction.Interface_ToggleFocus`
  (params (Focus :type Boolean))
  (`PrimitiveComponent.SetRenderCustomDepth` (`self.Vial`) Focus))

(event `/Game/Blueprints/BPI_Interaction.InterfaceInteract`
  (params (Player :type "/Game/FirstPerson/Blueprints/BP_FirstPersonCharacter Object Reference"))
  (bind _vial (`self.Vial`))
  (`/Engine/EditorBlueprintResources/StandardMacros.IsValid` (`/Game/FirstPerson/Blueprints/BP_FirstPersonCharacter.HeldItem` Player)
    (:`Is Not Valid`
      (`PrimitiveComponent.SetSimulatePhysics` _vial false)
      (`PrimitiveComponent.SetCollisionEnabled` _vial "NoCollision")
      (`/Game/UI/WBP_PlayerHUD.ShowDropUI` (`/Game/FirstPerson/Blueprints/BP_FirstPersonCharacter.HUDReference` Player))
      (`SceneComponent.K2_AttachToComponent` _vial (`/Game/FirstPerson/Blueprints/BP_FirstPersonCharacter.HoldPosition` Player) "None" "SnapToTarget" "SnapToTarget" "KeepWorld" true)
      (set `/Game/FirstPerson/Blueprints/BP_FirstPersonCharacter.HeldItem` self Player))))

(fn `GetInteractionWidgetRef`
  (returns (WidgetReference :type "WidgetComponent Object Reference"))
  (return (`self.Widget`)))

(fn `UserConstructionScript`)